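; Gate Blueprint that swings open when a Pawn overlaps its Box and reverses when a Pawn ends overlap with the actor.
; The GateOpenClose timeline drives the yaw of the Pivot component.
; A DoOnce limits the opening sound to one play per cycle.
; The timeline's Finished output, which follows both opening and reversing, plays the closing sound and resets that DoOnce through ResetGateSound.
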(event `self.Box.OnComponentBeginOverlap`
  (params (OverlappedComponent :type "PrimitiveComponent Object Reference") (OtherActor :type "Actor Object Reference") (OtherComp :type "PrimitiveComponent Object Reference") (OtherBodyIndex :type Integer) (bFromSweep :type Boolean) (SweepResult :type "HitResult Structure (by ref)"))
  (cast `Pawn` OtherActor)
  (`|ExecutionSequence`
    (:`then_0`
      (bind (_direction _gate_rotation) (`Timeline|Gate Open/Close` :!label _label)
        (:`Update`
          (`SceneComponent.K2_SetRelativeRotation` (`self.Pivot`) (`KismetMathLibrary.MakeRotator` 0.0 0.0 _gate_rotation) false false))
        (:`Finished`
          (`GameplayStatics.PlaySound2D` "/Game/Sounds/Gate_closing.Gate_closing" 50.0 1.0 0.0 null null)
          (`self.Reset Gate Sound`))))
    (:`then_1`
      (`/Engine/EditorBlueprintResources/StandardMacros.DoOnce` false :!label _label_2
        (:`Completed`
          (`GameplayStatics.PlaySound2D` "/Game/Sounds/Gate_opening.Gate_opening" 50.0 1.0 0.0 null null))))))

(event `Reset Gate Sound`
  (goto _label_2 :!via `Reset`))

(event `self.ReceiveActorEndOverlap`
  (params (OtherActor :type "Actor Object Reference"))
  (cast `Pawn` OtherActor)
  (goto _label :!via `Reverse`))

(fn `UserConstructionScript`)