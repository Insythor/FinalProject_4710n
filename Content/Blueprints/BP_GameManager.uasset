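; Game manager for a timed sheep-herding round that tracks the countdown and collected sheep.
; BeginPlay creates timer, counter and red-screen widgets, counts sheep, then runs a one-second delay loop that triggers a one-time camera shake and later red-screen fade near time-out.
; Sheep overlapping the herded barrier move to the shearing machine, increment the counter and are destroyed after a delay.
; Timeout sets EndOfGame, but the score-screen and quit logic is disconnected.
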(event `self.Sheep Herded Barrier.OnComponentBeginOverlap`
  (params (OverlappedComponent :type "PrimitiveComponent Object Reference") (OtherActor :type "Actor Object Reference") (OtherComp :type "PrimitiveComponent Object Reference") (OtherBodyIndex :type Integer) (bFromSweep :type Boolean) (SweepResult :type "HitResult Structure (by ref)"))
  ;[0 0 0] Disables sheep movement, and deletes them after x seconds
  ;;[1 0 0] *** WILL NEED TO BE CHANGED WHEN THE LEVEL IS MADE ***
  (bind _asbp_sheep_temp (cast `/Game/Blueprints/AI/NPC/BP_Sheep_TEMP` OtherActor))
  (`AIBlueprintHelperLibrary.SimpleMoveToActor` (`AIBlueprintHelperLibrary.GetAIController` _asbp_sheep_temp) (`self.Sheering Machine`))
  (`self.Update_CollectedSheep`)
  (`KismetSystemLibrary.Delay` (`self.Sheer Durration`))
  (`self.K2_DestroyActor` _asbp_sheep_temp))

(event `self.ReceiveBeginPlay`
  ;[0 0 0] Initializes UI and begins time loop
  ;;[1 0 0] *** CLASS OF SHEEP NEEDS TO BE CHANGED ***
  (`self.Initialize_UI_References`)
  ;;[1 0 0] *** Start Delay ***
  (`KismetSystemLibrary.Delay` 0.5)
  (`self.Loop Time`))

(event `Loop Time`
  ;[0 0 0] Updates the time UI
  (if (not (`self.End of Game`))
    (`KismetSystemLibrary.Delay` 1.0)
    (`self.Update_Time`)
    (`self.Loop Time`)))

(event `Timer Camera Shake`
  ;[0 0 0] Screen shake loop at 30s left, and red screen animation at 10s
  (`/Engine/EditorBlueprintResources/StandardMacros.DoOnce` false
    (:`Completed`
      (`GameplayStatics.PlayWorldCameraShake` "/Game/Blueprints/UI/TimerShake.TimerShake_C" (0.0 0.0 0.0) 1.0 2000000.0)
      (`KismetSystemLibrary.Delay` 20.0)
      (bind (_direction _opacity) (`Timeline|Time running out Red Screen Opacity` :!via `PlayFromStart`)
        (:`Update`
          (`Widget.SetRenderOpacity` (`self.RedScreen_UI`) _opacity))))))

(fn `Initialize_UI_References`
  (set `self.seconds` (`KismetStringLibrary.Conv_StringToInt` (`self.str_seconds`)))
  (set `self.minutes` (`KismetStringLibrary.Conv_StringToInt` (`self.str_minutes`)))
  (bind _returnvalue (`|CreateWidget` "/Game/Blueprints/UI/UI_Timer_BP.UI_Timer_BP_C"))
  (bind _output_get (set `self.Timer_UI` _returnvalue))
  (bind _returnvalue_2 (`|CreateWidget` "/Game/Blueprints/UI/UI_SheepCounter.UI_SheepCounter_C"))
  (bind _output_get_2 (set `self.SheepCounter_UI` _returnvalue_2))
  (`UserWidget.AddToViewport` _output_get 0)
  (`UserWidget.AddToViewport` _output_get_2 0)
  ;[1 0 0] *** NEEDS TO BE CHANGED WHEN SHEEP ARE IN GAME ***
  (bind _outactors (`GameplayStatics.GetAllActorsOfClass` "/Game/Blueprints/AI/NPC/BP_Sheep_TEMP.BP_Sheep_TEMP_C"))
  (set `self.Total Sheep` (`KismetArrayLibrary.Array_Length` _outactors))
  (bind _returnvalue_3 (`|CreateWidget` "/Game/Blueprints/UI/UI_RedScreen.UI_RedScreen_C"))
  (bind _output_get_3 (set `self.RedScreen_UI` _returnvalue_3))
  (`UserWidget.AddToViewport` _output_get_3 0)
  (`Widget.SetRenderOpacity` _output_get_3 0.0)
  (bind _outactors_2 (`GameplayStatics.GetAllActorsOfClass` "/Game/Blueprints/Environment/shearingMachine.shearingMachine_C"))
  (set `self.Sheering Machine` (`|GetArrayItem` _outactors_2)))

(fn `Update_CollectedSheep`
  ;[0 0 0] Adds +1 to the amount of Collected Sheep, and updates the UI
  (bind _result (`/Engine/EditorBlueprintResources/StandardMacros.IncrementInt` (`self.Collected Sheep`))
    (:`  `
      (`TextBlock.SetText` (`/Game/Blueprints/UI/UI_SheepCounter.SheepCollectedNumber` (`self.SheepCounter_UI`)) (`KismetTextLibrary.Conv_IntToText` _result)))))

(fn `Update_Time`
  (bind _returnvalue (`KismetStringLibrary.Conv_IntToString` (`self.seconds`)))
  (if (not (`self.End of Game`))
    ;[0 0 0] Triggers screen shake awhen there is 30s left in the round
    (if (and (<= (`self.seconds`) (`self.Camera Shake Start Time`)) (== (`self.minutes`) 0))
      (`self.Timer Camera Shake`))
    (bind _output_get (set `self.seconds` (- (`self.seconds`) 1)))
    (if (< (`self.seconds`) 0)
      (bind _output_get_2 (set `self.minutes` (- (`self.minutes`) 1)))
      (if (== _output_get_2 0)
        (set `self.str_minutes` ": ")
        (bind _output_get_3 (set `self.seconds` 59 :!label _label))
        (set `self.str_seconds` (`KismetStringLibrary.Conv_IntToString` _output_get_3))
        (elif (< (`self.minutes`) 0)
          (`KismetSystemLibrary.PrintString` "GameOver")
          (set `self.End of Game` true)
          (else
            (set `self.str_minutes` (`KismetStringLibrary.Concat_StrStr` (`KismetStringLibrary.Conv_IntToString` (`self.minutes`)) " :"))
            (goto _label))))
      (elif (< _output_get 10)
        (set `self.str_seconds` (`KismetStringLibrary.Concat_StrStr` "0" _returnvalue))
        (else
          (set `self.str_seconds` _returnvalue))))))

(fn `UserConstructionScript`)