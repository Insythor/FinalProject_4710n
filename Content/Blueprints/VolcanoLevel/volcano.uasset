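; Volcano actor that plays a looping rumble and continuously ejects pyroclast projectiles.
; BeginPlay starts the rumble audio, and its OnAudioFinished event restarts it.
; A DoOnce on that shared path launches a single self-repeating Delay loop, spawning a Pyroclast at the spawn-location component every three seconds.
; Each spawned mesh receives a force with random horizontal components and a fixed upward component.
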(event `self.Volcano_Rumble.OnAudioFinished`
  (`AudioComponent.Play` (`self.Volcano_Rumble`) 0.0 :!label _label)
  (`/Engine/EditorBlueprintResources/StandardMacros.DoOnce` false
    (:`Completed`
      (bind _returnvalue (`|SpawnActorFromClass` "/Game/Blueprints/VolcanoLevel/Pyroclast.Pyroclast_C" (`SceneComponent.K2_GetComponentToWorld` (`self.Pyroblast Spawn Location`)) "Undefined" "OverrideRootScale" null null :!label _label_2))
      (`PrimitiveComponent.AddForce` (`/Game/Blueprints/VolcanoLevel/Pyroclast.pyroclast01Mesh` _returnvalue) (`KismetMathLibrary.MakeVector` (`KismetMathLibrary.Conv_IntToDouble` (`KismetMathLibrary.RandomIntegerInRange` -5000000 5000000)) (`KismetMathLibrary.Conv_IntToDouble` (`KismetMathLibrary.RandomIntegerInRange` -5000000 5000000)) 30000.0) "None" false)
      (`KismetSystemLibrary.Delay` 3.0)
      (goto _label_2))))

(event `self.ReceiveBeginPlay`
  (goto _label))

(fn `UserConstructionScript`)