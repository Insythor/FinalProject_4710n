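; Volcano level pyroclast actor that swaps a solid mesh for a destructible one on impact, then despawns.
; The destructible starts query-only at BeginPlay and gains full physics collision when either component registers a hit.
; A hit on the mesh also stops its physics simulation and hides it without affecting child components, then destroys the actor after DespawnDelay.
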(event `self.ReceiveBeginPlay`
  (`PrimitiveComponent.SetCollisionEnabled` (`self.pyroClast01Destructible`) "QueryOnly"))

(event `self.pyroClast01Destructible.OnComponentHit`
  (params (HitComponent :type "PrimitiveComponent Object Reference") (OtherActor :type "Actor Object Reference") (OtherComp :type "PrimitiveComponent Object Reference") (NormalImpulse :type "Vector Structure") (Hit :type "HitResult Structure (by ref)"))
  (`PrimitiveComponent.SetCollisionEnabled` (`self.pyroClast01Destructible`) "QueryAndPhysics"))

(event `self.pyroclast01Mesh.OnComponentHit`
  (params (HitComponent :type "PrimitiveComponent Object Reference") (OtherActor :type "Actor Object Reference") (OtherComp :type "PrimitiveComponent Object Reference") (NormalImpulse :type "Vector Structure") (Hit :type "HitResult Structure (by ref)"))
  (`PrimitiveComponent.SetCollisionEnabled` (`self.pyroClast01Destructible`) "QueryAndPhysics")
  (`PrimitiveComponent.SetSimulatePhysics` (`self.pyroclast01Mesh`) false)
  (`SceneComponent.SetVisibility` (`self.pyroclast01Mesh`) false false)
  (`KismetSystemLibrary.Delay` (`self.despawnDelay`))
  (`self.K2_DestroyActor`))

(fn `UserConstructionScript`)