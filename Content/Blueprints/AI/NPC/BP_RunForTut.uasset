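; BP_RunForTut is a sheep NPC that wanders, flees when near the player dog or a fence, and stops fire effects on water overlap.
; Tick steers it directly away from the obstacle, which is the player when near a fence and the fence when near the player, and drives ABP_sheep's run flag.
; Bound events handle bark, which temporarily boosts speed and makes it follow the player, and delayed tick-off and destruction.
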(event `self.Water Collision.OnComponentBeginOverlap`
  (params (OverlappedComponent :type "PrimitiveComponent Object Reference") (OtherActor :type "Actor Object Reference") (OtherComp :type "PrimitiveComponent Object Reference") (OtherBodyIndex :type Integer) (bFromSweep :type Boolean) (SweepResult :type "HitResult Structure (by ref)"))
  (bind _onfireparticleeffect (`self.onFireParticleEffect`))
  ;[0 0 0] Puts out fire
  (cast `/Game/Blueprints/Items/waterCollision` OtherActor)
  (if (`ActorComponent.IsActive` _onfireparticleeffect)
    (`ActorComponent.SetActive` _onfireparticleeffect false false)))

(event `self.ReceiveBeginPlay`
  ;[0 0 0] Begin Play
  (`CharacterMovementComponent.SetAvoidanceEnabled` (`self.CharacterMovement`) true)
  ;;[0 0 0] Called from the Player, increases movement speed after bark, then resets it back after 5 seconds
  (add `self.Increase Movement Speed` (delegate `Bark Movement`))
  ;;[0 0 0] Disables tick so that the sheep don't move once sheered,then kills them after 5s
  (add `self.Disable Tick and Kill` (delegate `Tick Off and Kill`)))

(event `Bark Movement` :!signature `self.Increase Movement Speed`
  (params (`Bark Movement Speed` :type "Float (double-precision)") (`Bark Duration` :type "Float (double-precision)"))
  ;[0 0 0] Begin Play
  ;;[0 0 0] Called from the Player, increases movement speed after bark, then resets it back after 5 seconds
  (set `self.Bark Movement Increase` `Bark Movement Speed`)
  (set `self.Bark Duration` `Bark Duration`)
  (set `self.speed` (+ (`self.speed`) (`self.Bark Movement Increase`)))
  (set `self.follow?` true)
  (`KismetSystemLibrary.Delay` (`self.Bark Duration`))
  (set `self.speed` (- (`self.speed`) (`self.Bark Movement Increase`)))
  (set `self.follow?` false))

(event `Tick Off and Kill`
  ;[0 0 0] Begin Play
  ;;[0 0 0] Disables tick so that the sheep don't move once sheered,then kills them after 5s
  (`KismetSystemLibrary.Delay` 0.2)
  (`self.SetActorTickEnabled` false)
  (`KismetSystemLibrary.Delay` 5.0)
  (`self.K2_DestroyActor`))

(event `self.ReceiveTick`
  (params (DeltaSeconds :type "Float (single-precision)"))
  (bind _returnvalue (`KismetMathLibrary.RandomInteger` 200))
  (bind _returnvalue_2 (`GameplayStatics.GetPlayerCharacter` 0))
  (bind (_returnvalue_x _returnvalue_y _returnvalue_z _returnrotator) (`self.GetRunDirection` (`self.currentObstacle`) DeltaSeconds))
  (bind (_returnvalue_x_2 _returnvalue_y_2) (`KismetMathLibrary.BreakVector` (`self.K2_GetActorLocation` self)))
  (bind _returnvalue_3 (< (`self.GetDistanceTo` _returnvalue_2 self) (`self.distancetodog`)))
  (`self.Animation` self)
  (if (`self.follow?`)
    (`|AIMoveTo` self (`self.K2_GetActorLocation` _returnvalue_2) _returnvalue_2)
    (else
      ;[0 0 0] Checks the distance from the sheep to the fence, if it's within "Distance To Fence"
      ; set the fence as the current obstacle
      (for _array_element (`self.Fence Array`)
        (`/Engine/EditorBlueprintResources/StandardMacros.IsValid` _returnvalue_2
          (:`Is Valid`
            (bind _returnvalue_4 (< (`self.GetDistanceTo` _array_element self) (`self.distancetofence`)))
            (set `self.moving?` (or _returnvalue_4 _returnvalue_3)) ; If the sheep is within either\nDistance To Dog or the Fence\nSet Moving to True
            ;[0 0 0] Sets the current obstable to either the player or a fence post
            (if _returnvalue_4
              (set `self.currentObstacle` (`GameplayStatics.GetPlayerCharacter` 0))
              (`/Engine/EditorBlueprintResources/StandardMacros.IsValid` (`self.currentObstacle`) :!label _label
                (:`Is Valid`
                  (`self.K2_SetActorLocation` (`KismetMathLibrary.MakeVector` _returnvalue_x _returnvalue_y _returnvalue_z) true)
                  (`self.K2_SetActorRotation` (`KismetMathLibrary.RInterpTo` (`self.K2_GetActorRotation`) _returnrotator (`GameplayStatics.GetWorldDeltaSeconds`) 10.0))
                  (set `self.DoneWander?` true)))
              (elif _returnvalue_3
                (set `self.currentObstacle` _array_element)
                (goto _label)
                (elif (`self.DoneWander?`)
                  (set `self.DoneWander?` false)
                  (`|AIMoveTo` self (`KismetMathLibrary.MakeVector` (+ _returnvalue_x_2 (`KismetMathLibrary.Conv_IntToDouble` (- _returnvalue 100))) (+ _returnvalue_y_2 (`KismetMathLibrary.Conv_IntToDouble` (- (`KismetMathLibrary.RandomInteger` 200) 100)))) null (`KismetMathLibrary.Conv_IntToDouble` _returnvalue)
                    (:`OnSuccess`
                      _)
                    (:`OnFail`
                      _))
                  (set `self.DoneWander?` true))))))))))

(fn `Animation`
  (bind _returnvalue (`SkeletalMeshComponent.GetAnimInstance` (`self.Mesh`)))
  (if (`self.moving?`)
    (bind _asabp_sheep (cast `/Game/Assets/Animations/sheep/ABP_sheep` _returnvalue))
    (set `/Game/Assets/Animations/sheep/ABP_sheep.canrun` true _asabp_sheep)
    (else
      (bind _asabp_sheep_2 (cast `/Game/Assets/Animations/sheep/ABP_sheep` _returnvalue))
      (set `/Game/Assets/Animations/sheep/ABP_sheep.canrun` false _asabp_sheep_2))))

(fn `GetRunDirection`
  (params (`Current Obstacle` :type "Actor Object Reference") (`Delta Seconds` :type "Float (double-precision)"))
  (returns (ReturnValue_X :type "Float (double-precision)") (ReturnValue_Y :type "Float (double-precision)") (ReturnValue_Z :type "Float (double-precision)") (ReturnRotator :type "Rotator Structure"))
  (bind _returnvalue (`self.K2_GetActorLocation` `Current Obstacle`))
  (bind _returnvalue_2 (`self.K2_GetActorLocation`))
  (bind (_returnvalue_roll _returnvalue_pitch _returnvalue_yaw) (`KismetMathLibrary.BreakRotator` (`KismetMathLibrary.FindLookAtRotation` _returnvalue _returnvalue_2)))
  (bind (_returnvalue_x _returnvalue_y) (`KismetMathLibrary.BreakVector` (+ (* (* (`KismetMathLibrary.Normal` (- _returnvalue_2 _returnvalue)) `Delta Seconds`) (`self.speed`)) _returnvalue_2)))
  (return _returnvalue_x _returnvalue_y (.z _returnvalue_2) (`KismetMathLibrary.MakeRotator` 0.0 0.0 _returnvalue_yaw)))

(fn `UserConstructionScript`
  (bind _outactors (`GameplayStatics.GetAllActorsOfClass` "/Game/Blueprints/Environment/BP_fence.BP_fence_C"))
  (set `self.Fence Array` _outactors))