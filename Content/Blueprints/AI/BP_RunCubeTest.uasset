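; BP_RunCubeTest is an AI test actor that flees from the player.
; Each tick, while player character 0 is within a fixed radius, it moves directly away at constant speed, scaled by delta time.
; Movement uses SetActorLocation along the normalized player-to-actor direction and keeps the current height, with no navigation or pathfinding.
; A node chain that would yaw it to face the player is present but never runs.
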(event `self.ReceiveTick`
  (params (DeltaSeconds :type "Float (single-precision)"))
  (bind _returnvalue (`self.K2_GetActorLocation`))
  (bind _returnvalue_2 (`GameplayStatics.GetPlayerCharacter` 0))
  (bind (_returnvalue_x _returnvalue_y) (`KismetMathLibrary.BreakVector` (+ (* (* (`KismetMathLibrary.Normal` (- _returnvalue (`self.K2_GetActorLocation` _returnvalue_2))) DeltaSeconds) 500.0) _returnvalue)))
  (if (< (`self.GetDistanceTo` _returnvalue_2 self) 1000.0)
    (`self.K2_SetActorLocation` (`KismetMathLibrary.MakeVector` _returnvalue_x _returnvalue_y (.z _returnvalue)))))

(fn `UserConstructionScript`)