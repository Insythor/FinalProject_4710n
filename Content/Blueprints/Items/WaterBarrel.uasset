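; Water barrel item that acts as a limited-duration fire hose, with a water jet particle effect and looping-style hose sound.
; Spray_Hose, bound to a SprayWater event, toggles jet and sound, then after a delay reduces the remaining duration.
; Each spray launches an invisible-purpose WaterCollision cube forward by physics force to detect water hits, widened to hit sheep more easily.
; When time runs out, the barrel hides, silences and destroys itself.
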(event `self.ReceiveBeginPlay`
  (add `self.Spray Water` (delegate `Spray_Hose`))
  ;[0.5 0 1] Spawn the Spraying Water Sound, then turns it off so it's not playing all game
  (bind _returnvalue (`GameplayStatics.SpawnSound2D` "/Game/Sounds/Hose_sound.Hose_sound" (`self.Water Volume`) 1.0 0.0 null false false))
  (`ActorComponent.Deactivate` _returnvalue))

(event `Spray_Hose` :!signature `self.Spray Water`
  (params (SprayWater :type Boolean))
  (bind _waterjet (`self.WaterJet`))
  (bind (_returnvalue_location _returnvalue_rotation) (`KismetMathLibrary.BreakTransform` (`SceneComponent.K2_GetComponentToWorld` (`self.DefaultSceneRoot`))))
  ;[0 0 0] Updates the amount of time left on the fire hose, and toggles particle system
  (if (and SprayWater (`self.Can Spray?`))
    (`ActorComponent.Activate` _waterjet false)
    ;;[0.5 0 1] Water sounds
    (`ActorComponent.Activate` (stale `self.ReceiveBeginPlay` _returnvalue) false)
    (`KismetSystemLibrary.Delay` (`self.Spray Frequency`))
    (bind _output_get (set `self.Spray Duration` (- (`self.Spray Duration`) (`self.Spray Frequency`))))
    (`KismetSystemLibrary.PrintString` (`KismetStringLibrary.Conv_DoubleToString` _output_get)) ; Printing duration left on hose
    ;[0 0 0] Spawns a Cube and adds force to it. This is for knowing if something is being hit by water
    (bind _returnvalue (`|SpawnActorFromClass` "/Game/Blueprints/Items/waterCollision.waterCollision_C" (`KismetMathLibrary.MakeTransform` _returnvalue_location _returnvalue_rotation (0.1 0.5 0.1)) "Undefined" "OverrideRootScale" null null)) ; Wider cube make it a bit easier to hit the sheep
    (`PrimitiveComponent.AddForce` (`/Game/Blueprints/Items/waterCollision.Cube` _returnvalue) (* (`SceneComponent.GetForwardVector` (`self.DefaultSceneRoot`)) 100000.0) "None" false)
    ;[0 0 0] Delete Fire Hose and Deactivate particle system when time is up
    (if (<= (`self.Spray Duration`) 0.0)
      (set `self.Can Spray?` false)
      (`ActorComponent.Deactivate` (`self.WaterJet`))
      (`SceneComponent.SetHiddenInGame` (`self.Barrel`) true false) ; Shitty System but it works
      (`self.Deactivate Water`)
      (`KismetSystemLibrary.Delay` 3.0)
      (`self.K2_DestroyActor`)
      (else
        (set `self.Can Spray?` true)))
    (else
      (`ActorComponent.Deactivate` _waterjet)
      (`ActorComponent.Deactivate` (stale `self.ReceiveBeginPlay` _returnvalue) :!label _label))))

(event `Deactivate Water`
  (goto _label))

(fn `UserConstructionScript`)