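; Fire hose item whose nozzle extends, retracts and sprays water, driven by player input through a dispatcher from ThirdPersonCharacter.
; Nozzle movement is clamped, swept and updates the cable length.
; Spraying activates a particle jet and, after a delay, drains duration and launches a physics-pushed WaterCollision actor from the nozzle.
; When duration runs out, the hose hides its meshes and cable, then destroys itself after a short delay.
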(event `self.ReceiveBeginPlay`
  (add `self.Move Hose` (delegate `FireHose_Use`)) ; Dispatcher is comming from \nThirdPersonCharacter
)

(event `FireHose_Use` :!signature `self.Move Hose`
  (params (`Hose Out` :type Boolean) (`Hose In` :type Boolean) (`Use Hose` :type Boolean))
  (bind _nozzleholder (`self.NozzleHolder`))
  (bind _water_jet (`self.Water Jet`))
  (bind _relativelocation_x (`KismetMathLibrary.BreakVector` (`SceneComponent.RelativeLocation` _nozzleholder)))
  (bind _relativelocation_x_2 (`KismetMathLibrary.BreakVector` (`SceneComponent.RelativeLocation` (`self.Root`))))
  ;[0 0 0] Move the nozzle in/out on tick, based on player input
  (if `Hose Out`
    (set `self.TEMP_Hose X Location` (`KismetMathLibrary.FClamp` (+ _relativelocation_x (`self.Nozzle Movement Speed`)) 0.0 (`self.Max Nozzle Distance`)))
    (`SceneComponent.K2_SetRelativeLocation` _nozzleholder (`KismetMathLibrary.MakeVector` (`self.TEMP_Hose X Location`) 50.0) true false :!label _label)
    ;[0 0 0] Changes the hose length based on the distance to nozzle
    (set `CableComponent.CableLength` (- _relativelocation_x_2 (.x (.location (`SceneComponent.GetRelativeTransform` (`self.NozzleHolder`))))) (`self.Cable`))
    ;[1 0 0] Debugging / Playtesting: Prints when the Nozzle is at max distance
    (if (== (`self.TEMP_Hose X Location`) (`self.Max Nozzle Distance`))
      (`/Engine/EditorBlueprintResources/StandardMacros.DoOnce` false :!label _label_2
        (:`Completed`
          (`KismetSystemLibrary.PrintString` "HOSE HAS REACHED MAX RANGE! " true true (struct :`R` 1.0 :`A` 1.0) 4.0)))
      (else
        (goto _label_2 :!via `Reset`)))
    (elif `Hose In`
      (set `self.TEMP_Hose X Location` (`KismetMathLibrary.FClamp` (- _relativelocation_x (`self.Nozzle Movement Speed`)) 50.0 (`self.Max Nozzle Distance`)))
      (goto _label)
      (else
        ;[0 0 0] Updates the amount of time left on the fire hose, and toggles particle system
        (if (and `Use Hose` (`self.Can Spray?`))
          (`ActorComponent.Activate` _water_jet false)
          (`KismetSystemLibrary.Delay` (`self.Spray Frequency`))
          (bind _output_get (set `self.Hose Duration` (- (`self.Hose Duration`) (`self.Spray Frequency`))))
          (`KismetSystemLibrary.PrintString` (`KismetStringLibrary.Conv_DoubleToString` _output_get)) ; Printing duration left on hose
          (bind _returnvalue (`|SpawnActorFromClass` "/Game/Blueprints/Items/waterCollision.waterCollision_C" (`SceneComponent.K2_GetComponentToWorld` (`self.fireHoseNozzleMesh`)) "Undefined" "OverrideRootScale" null null))
          (`PrimitiveComponent.AddForce` (`/Game/Blueprints/Items/waterCollision.Cube` _returnvalue) (* (`SceneComponent.GetForwardVector` (`self.fireHoseBaseMesh`)) 400000.0) "None" false)
          ;[0 0 0] Delete Fire Hose and Deactivate particle system when time is up
          (if (<= (`self.Hose Duration`) 0.0)
            (set `self.Can Spray?` false)
            (`SceneComponent.SetHiddenInGame` (`self.Cable`) true false)
            (`SceneComponent.SetHiddenInGame` (`self.fireHoseNozzleMesh`) true false)
            (`SceneComponent.SetHiddenInGame` (`self.fireHoseBaseMesh`) true false) ; Shitty System but it works
            (`KismetSystemLibrary.Delay` 3.0)
            (`self.K2_DestroyActor`)
            (else
              (set `self.Can Spray?` true)))
          (else
            (`ActorComponent.Deactivate` _water_jet)))))))

(fn `UserConstructionScript`
  (bind _nozzleholder (`self.NozzleHolder`))
  ;[0 0 0] Binds the Nozzle head to the Nozzle Holder
  (`SceneComponent.K2_AttachToComponent` (`self.fireHoseNozzleMesh`) _nozzleholder (`|GetArrayItem` (`SceneComponent.GetAllSocketNames` _nozzleholder)) "SnapToTarget" "KeepRelative" "KeepRelative" true)
  (`self.SetActorTickEnabled` false))