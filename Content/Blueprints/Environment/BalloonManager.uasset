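; Manages wool balloons that spawn at a start point, rise to a midpoint, then drift to the Zeppelin.
; A bound SpawnWool event spawns randomly scaled Wool; start, mid and end overlaps add it to MoveUp, shift it to MoveToZeppelin, then destroy it.
; Tick eases each array toward its target by a fraction of remaining distance, with one axis clamped to limit speed.
; Tick runs only while balloons are in flight.
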(event `self.End Location.OnComponentBeginOverlap`
  (params (OverlappedComponent :type "PrimitiveComponent Object Reference") (OtherActor :type "Actor Object Reference") (OtherComp :type "PrimitiveComponent Object Reference") (OtherBodyIndex :type Integer) (bFromSweep :type Boolean) (SweepResult :type "HitResult Structure (by ref)"))
  (bind _move_to_zeppelin (`self.Move to Zeppelin`))
  ;[0 0 0] Array Managment
  ;;[0 0 0] Deletes the Balloons once they get to the Zeppelin and removes them form the array
  (`self.K2_DestroyActor` OtherActor)
  (`KismetArrayLibrary.Array_Remove` _move_to_zeppelin (`KismetArrayLibrary.Array_Find` _move_to_zeppelin OtherActor))
  ;;[0 0 0] Disables tick if no balloons are in the game
  (if (== (+ (`KismetArrayLibrary.Array_Length` (`self.Move Up`)) (`KismetArrayLibrary.Array_Length` (`self.Move to Zeppelin`))) 0) :!label _label
    (`self.SetActorTickEnabled` false)))

(event `self.ReceiveTick`
  (params (DeltaSeconds :type "Float (single-precision)"))
  (bind _move_up (`self.Move Up`))
  (bind _move_to_zeppelin (`self.Move to Zeppelin`))
  ;[0 0 0] Moves the Wool to the Zeppelin
  ;;[0 0 0] Moves the balloons up
  (`|ExecutionSequence`
    (:`then_0`
      (for (_ _array_index) _move_up
        (bind _output (`|GetArrayItem` _move_up _array_index))
        (bind _returnvalue (`self.K2_GetActorLocation` _output))
        (bind (_returnvalue_x _returnvalue_y _returnvalue_z) (`KismetMathLibrary.BreakVector` (/ (- _returnvalue (`SceneComponent.K2_GetComponentLocation` (`self.Mid Location`))) 98.0)))
        (`self.K2_SetActorRelativeLocation` _output (- _returnvalue (`KismetMathLibrary.MakeVector` _returnvalue_x _returnvalue_y (`KismetMathLibrary.FClamp` _returnvalue_z -1.0 0.0))) false false)))
    (:`then_1`
      ;;[0 0 0] Moves the balloons to the zeppelin
      (for (_ _array_index_2) _move_to_zeppelin
        (bind _output_2 (`|GetArrayItem` _move_to_zeppelin _array_index_2))
        (bind _returnvalue_2 (`self.K2_GetActorLocation` _output_2))
        (bind (_returnvalue_x_2 _returnvalue_y_2 _returnvalue_z_2) (`KismetMathLibrary.BreakVector` (/ (- _returnvalue_2 (`SceneComponent.K2_GetComponentLocation` (`self.End Location`))) 90.0)))
        (`self.K2_SetActorRelativeLocation` _output_2 (- _returnvalue_2 (`KismetMathLibrary.MakeVector` _returnvalue_x_2 (`KismetMathLibrary.FClamp` _returnvalue_y_2 -2.0 0.0) _returnvalue_z_2)) false false)))))

(event `self.Mid Location.OnComponentBeginOverlap`
  (params (OverlappedComponent :type "PrimitiveComponent Object Reference") (OtherActor :type "Actor Object Reference") (OtherComp :type "PrimitiveComponent Object Reference") (OtherBodyIndex :type Integer) (bFromSweep :type Boolean) (SweepResult :type "HitResult Structure (by ref)"))
  (bind _move_up (`self.Move Up`))
  ;[0 0 0] Array Managment
  ;;[0 0 0] Removes the wool from the array when it reaches the mid location
  (`KismetArrayLibrary.Array_Remove` _move_up (`KismetArrayLibrary.Array_Find` _move_up OtherActor))
  (`KismetArrayLibrary.Array_AddUnique` (`self.Move to Zeppelin`) OtherActor)
  (goto _label))

(event `self.Start Location.OnComponentBeginOverlap`
  (params (OverlappedComponent :type "PrimitiveComponent Object Reference") (OtherActor :type "Actor Object Reference") (OtherComp :type "PrimitiveComponent Object Reference") (OtherBodyIndex :type Integer) (bFromSweep :type Boolean) (SweepResult :type "HitResult Structure (by ref)"))
  ;[0 0 0] Array Managment
  ;;[0 0 0] Adds the wool to the array on spawn, and enables tick
  (`KismetArrayLibrary.Array_AddUnique` (`self.Move Up`) OtherActor)
  (`self.SetActorTickEnabled` true))

(event `self.ReceiveBeginPlay`
  ;[0 0 0] Called in the Sheering machine, spawn wool
  (add `self.Spawn Wool` (delegate `SpawnWool`))
  (`self.SetActorTickEnabled` false))

(event `SpawnWool`
  (bind _returnvalue (`KismetMathLibrary.RandomFloatInRange` 0.6 0.8))
  (bind (_returnvalue_location _returnvalue_rotation) (`KismetMathLibrary.BreakTransform` (`SceneComponent.K2_GetComponentToWorld` (`self.Start Location`))))
  ;[0 0 0] Called in the Sheering machine, spawn wool
  (`|SpawnActorFromClass` "/Game/Blueprints/Environment/Wool.Wool_C" (`KismetMathLibrary.MakeTransform` _returnvalue_location _returnvalue_rotation (`KismetMathLibrary.MakeVector` _returnvalue _returnvalue _returnvalue)) "AlwaysSpawn" "OverrideRootScale" null null :!label _label_2))

(event `Spawn Wool Debugg`
  ;[0 0 0] Called in the Sheering machine, spawn wool
  (goto _label_2))

(fn `UserConstructionScript`)